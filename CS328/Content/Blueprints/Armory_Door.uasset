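; Armory door actor that the player opens and closes with the Interact input while holding a key.
; A Box overlap sets an in-range flag and enables or disables the actor's input for player-controlled characters.
; Interact checks range and the first-person character's HasKey, then toggles between open and closed by easing the Cube to a new transform.
; Input is disabled during the move, and the Box is then repositioned to follow the door.
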(event `self.Box.OnComponentEndOverlap`
  (params (OverlappedComponent :type "PrimitiveComponent Object Reference") (OtherActor :type "Actor Object Reference") (OtherComp :type "PrimitiveComponent Object Reference") (OtherBodyIndex :type Integer))
  (bind _ascharacter (cast `Character` OtherActor))
  (if (`Pawn.IsPlayerControlled` _ascharacter)
    (set `self.In Range` false)
    (`self.DisableInput` (`GameplayStatics.GetPlayerController` 0))))

(event `self.Box.OnComponentBeginOverlap`
  (params (OverlappedComponent :type "PrimitiveComponent Object Reference") (OtherActor :type "Actor Object Reference") (OtherComp :type "PrimitiveComponent Object Reference") (OtherBodyIndex :type Integer) (bFromSweep :type Boolean) (SweepResult :type "HitResult Structure (by ref)"))
  (bind _ascharacter (cast `Character` OtherActor))
  (if (`Pawn.IsPlayerControlled` _ascharacter)
    (set `self.In Range` true)
    (`self.EnableInput` (`GameplayStatics.GetPlayerController` 0))))

(event `InputAction|Interact`
  (params (Key :type "Key Structure"))
  (bind _returnvalue (`GameplayStatics.GetPlayerController` 0))
  (bind _returnvalue_2 (`GameplayStatics.GetPlayerController` 0))
  (:`Pressed`
    (if (and (`self.In Range`) (`/Game/FirstPersonBP/Blueprints/FirstPersonCharacter.HasKey` (cast `/Game/FirstPersonBP/Blueprints/FirstPersonCharacter` (`GameplayStatics.GetPlayerCharacter` 0) :!pure true)))
      (if (`self.Is Closed`)
        (set `self.Is Closed` false)
        (`self.DisableInput` _returnvalue)
        (`KismetSystemLibrary.MoveComponentTo` (`self.Cube`) (140.0 -30.0 200.0) (struct :`Yaw` 90.0) true true 0.5)
        (`self.EnableInput` _returnvalue_2)
        (`KismetSystemLibrary.MoveComponentTo` (`self.Box`) (150.0 -30.0 220.0) (struct) false false 0.0)
        (else
          (set `self.Is Closed` true)
          (`self.DisableInput` _returnvalue)
          (`KismetSystemLibrary.MoveComponentTo` (`self.Cube`) (-10.0 -180.0 200.0) (struct) false true 0.5)
          (`self.EnableInput` _returnvalue_2)
          (`KismetSystemLibrary.MoveComponentTo` (`self.Box`) (0.0 -180.0 220.0) (struct) false false 0.0))))))

(fn `UserConstructionScript`)