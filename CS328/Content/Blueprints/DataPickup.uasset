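; DataPickup is an interactable laptop that the player reads once to collect data.
; A box overlap toggles input and a tooltip for the player-controlled character, enabling the Interact action only in range.
; Interacting removes the box, swaps the open laptop for a closed mesh and calls GetData on the player character and the first Exit_Door found at BeginPlay.
; It also plays a sound and shows a temporary DataLore widget.
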(event `self.ReceiveBeginPlay`
  (bind _outactors (`GameplayStatics.GetAllActorsOfClass` "/Game/Blueprints/Exit_Door.Exit_Door_C"))
  (set `self.Exit` (`|GetArrayItem` _outactors)))

(event `self.Box.OnComponentEndOverlap`
  (params (OverlappedComponent :type "PrimitiveComponent Object Reference") (OtherActor :type "Actor Object Reference") (OtherComp :type "PrimitiveComponent Object Reference") (OtherBodyIndex :type Integer))
  (bind _ascharacter (cast `Character` OtherActor))
  (if (`Pawn.IsPlayerControlled` _ascharacter)
    (`self.DisableInput` (`GameplayStatics.GetPlayerController` 0))
    (`SceneComponent.SetVisibility` (`self.Tooltip`) false false)))

(event `self.Box.OnComponentBeginOverlap`
  (params (OverlappedComponent :type "PrimitiveComponent Object Reference") (OtherActor :type "Actor Object Reference") (OtherComp :type "PrimitiveComponent Object Reference") (OtherBodyIndex :type Integer) (bFromSweep :type Boolean) (SweepResult :type "HitResult Structure (by ref)"))
  (bind _ascharacter (cast `Character` OtherActor))
  (if (`Pawn.IsPlayerControlled` _ascharacter)
    (`self.EnableInput` (`GameplayStatics.GetPlayerController` 0))
    (`SceneComponent.SetVisibility` (`self.Tooltip`) true false)))

(event `InputAction|Interact`
  (params (Key :type "Key Structure"))
  (:`Pressed`
    (if (`self.Unread`)
      (set `self.Unread` false)
      (`self.DisableInput` (`GameplayStatics.GetPlayerController` 0))
      (`ActorComponent.K2_DestroyComponent` (`self.Box`))
      (`ActorComponent.K2_DestroyComponent` (`self.SM_Laptop`))
      (`SceneComponent.SetVisibility` (`self.SM_Laptop_Closed`) true false)
      (`/Game/FirstPersonBP/Blueprints/FirstPersonCharacter.Get Data` (cast `/Game/FirstPersonBP/Blueprints/FirstPersonCharacter` (`GameplayStatics.GetPlayerCharacter` 0) :!pure true))
      (`/Game/Blueprints/Exit_Door.GetData` (`self.Exit`))
      (`GameplayStatics.PlaySound2D` "/Game/Sounds/Data/data.data" 1.0 1.0 0.0 null null)
      (bind _returnvalue (`|CreateWidget` "/Game/Widgets/DataLore.DataLore_C"))
      (`UserWidget.AddToViewport` _returnvalue 0)
      (`KismetSystemLibrary.Delay` 7.0)
      (`Widget.RemoveFromParent` _returnvalue))))

(fn `UserConstructionScript`)