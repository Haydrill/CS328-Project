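; Sliding door Blueprint that moves two panels, Cube2 and Cube3, along X between two positions using MoveComponentTo.
; Overlap counters Ctr2 and Ctr3 trigger a move only on reaching one when incrementing or zero when decrementing.
; The triggers are crossed: entering Box shifts Cube2 and leaving Box1 returns it, while entering Box1 shifts Cube3 and leaving Box returns it.
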(event `self.Box1.OnComponentBeginOverlap`
  (params (OverlappedComponent :type "PrimitiveComponent Object Reference") (OtherActor :type "Actor Object Reference") (OtherComp :type "PrimitiveComponent Object Reference") (OtherBodyIndex :type Integer) (bFromSweep :type Boolean) (SweepResult :type "HitResult Structure (by ref)"))
  (bind _output_get (set `self.Ctr3` (+ (`self.Ctr3`) 1)))
  (if (== _output_get 1)
    (`KismetSystemLibrary.MoveComponentTo` (`self.Cube3`) (-750.0 60.0 200.0))))

(event `self.Box.OnComponentBeginOverlap`
  (params (OverlappedComponent :type "PrimitiveComponent Object Reference") (OtherActor :type "Actor Object Reference") (OtherComp :type "PrimitiveComponent Object Reference") (OtherBodyIndex :type Integer) (bFromSweep :type Boolean) (SweepResult :type "HitResult Structure (by ref)"))
  (bind _output_get (set `self.Ctr2` (+ (`self.Ctr2`) 1)))
  (if (== _output_get 1)
    (`KismetSystemLibrary.MoveComponentTo` (`self.Cube2`) (-130.0 60.0 200.0))))

(event `self.Box.OnComponentEndOverlap`
  (params (OverlappedComponent :type "PrimitiveComponent Object Reference") (OtherActor :type "Actor Object Reference") (OtherComp :type "PrimitiveComponent Object Reference") (OtherBodyIndex :type Integer))
  (bind _output_get (set `self.Ctr3` (- (`self.Ctr3`) 1)))
  (if (== _output_get 0)
    (`KismetSystemLibrary.MoveComponentTo` (`self.Cube3`) (-560.0 60.0 200.0))))

(event `self.Box1.OnComponentEndOverlap`
  (params (OverlappedComponent :type "PrimitiveComponent Object Reference") (OtherActor :type "Actor Object Reference") (OtherComp :type "PrimitiveComponent Object Reference") (OtherBodyIndex :type Integer))
  (bind _output_get (set `self.Ctr2` (- (`self.Ctr2`) 1)))
  (if (== _output_get 0)
    (`KismetSystemLibrary.MoveComponentTo` (`self.Cube2`) (-310.0 60.0 200.0))))

(fn `UserConstructionScript`)