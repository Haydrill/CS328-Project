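; Player controller Blueprint that toggles the pause menu on the Pause input action.
; With no menu open, it creates and displays the pause widget, switches to game-and-UI input with a visible cursor, pauses the game and hides the FirstPersonCharacter HUD.
; Pressing again removes and clears the stored widget reference, restores game-only input, hides the cursor, unpauses and shows the HUD.
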(event `InputAction|Pause` :paused true
  (params (Key :type "Key Structure"))
  (bind _returnvalue (`GameplayStatics.GetPlayerController` 0))
  (bind _pauseuiref (`self.PauseUIRef`))
  (bind _asfirst_person_character (cast `/Game/FirstPersonBP/Blueprints/FirstPersonCharacter` (`GameplayStatics.GetPlayerCharacter` 0) :!pure true))
  (:`Pressed`
    (`/Engine/EditorBlueprintResources/StandardMacros.IsValid` _pauseuiref
      (:`Is Valid`
        (`Widget.RemoveFromParent` _pauseuiref)
        (set `self.PauseUIRef` null)
        (`WidgetBlueprintLibrary.SetInputMode_GameOnly` _returnvalue)
        (set `self.bShowMouseCursor` false)
        (`GameplayStatics.SetGamePaused` false)
        (`/Game/FirstPersonBP/Blueprints/FirstPersonCharacter.ToggleHUDon` _asfirst_person_character))
      (:`Is Not Valid`
        (bind _returnvalue_2 (`|CreateWidget` "/Game/Widgets/PauseMenu.PauseMenu_C"))
        (bind _output_get (set `self.PauseUIRef` _returnvalue_2))
        (`UserWidget.AddToViewport` _output_get 0)
        (`WidgetBlueprintLibrary.SetInputMode_GameAndUIEx` _returnvalue null)
        (set `PlayerController.bShowMouseCursor` true _returnvalue)
        (`GameplayStatics.SetGamePaused` true)
        (`/Game/FirstPersonBP/Blueprints/FirstPersonCharacter.ToggleHUDoff` _asfirst_person_character)))))

(fn `UserConstructionScript`)