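; Exit door Blueprint that opens once data has been collected five times.
; Each GetData event call increments a counter.
; When the counter reaches five, the Cube and Red components are destroyed and the ToolTip is hidden.
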(event `GetData`
  (bind _output_get (set `self.Data` (+ (`self.Data`) 1)))
  (if (== _output_get 5)
    (`ActorComponent.K2_DestroyComponent` (`self.Cube`))
    (`ActorComponent.K2_DestroyComponent` (`self.Red`))
    (`SceneComponent.SetVisibility` (`self.ToolTip`) false false)))

(fn `UserConstructionScript`)