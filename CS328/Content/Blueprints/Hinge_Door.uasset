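; Hinged door that the player opens and closes with Interact while inside its Box trigger, and that non-player characters open automatically on entering.
; Overlap events toggle player input and two tooltips, which appear only when the player enters while it is closed.
; MoveComponentTo eases the Cube between preset transforms and relocates the trigger with it, pausing input around the swing.
; An Underwater flag slows the movement.
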(event `self.Box.OnComponentEndOverlap`
  (params (OverlappedComponent :type "PrimitiveComponent Object Reference") (OtherActor :type "Actor Object Reference") (OtherComp :type "PrimitiveComponent Object Reference") (OtherBodyIndex :type Integer))
  (bind _ascharacter (cast `Character` OtherActor))
  (if (`Pawn.IsPlayerControlled` _ascharacter)
    (set `self.In Range` false)
    (`self.DisableInput` (`GameplayStatics.GetPlayerController` 0))
    (`SceneComponent.SetVisibility` (`self.InteractTooltip`) false false)
    (`SceneComponent.SetVisibility` (`self.InteractTooltip1`) false false)))

(event `self.Box.OnComponentBeginOverlap`
  (params (OverlappedComponent :type "PrimitiveComponent Object Reference") (OtherActor :type "Actor Object Reference") (OtherComp :type "PrimitiveComponent Object Reference") (OtherBodyIndex :type Integer) (bFromSweep :type Boolean) (SweepResult :type "HitResult Structure (by ref)"))
  (bind _returnvalue (`KismetMathLibrary.SelectFloat` 2.0 0.5 (`self.Underwater`)))
  (bind _ascharacter (cast `Character` OtherActor))
  (if (`Pawn.IsPlayerControlled` _ascharacter)
    (set `self.In Range` true)
    (`self.EnableInput` (`GameplayStatics.GetPlayerController` 0))
    (if (`self.Is Closed`)
      (`SceneComponent.SetVisibility` (`self.InteractTooltip`) true false)
      (`SceneComponent.SetVisibility` (`self.InteractTooltip1`) true false)
      (else
        (`SceneComponent.SetVisibility` (`self.InteractTooltip`) false false)
        (`SceneComponent.SetVisibility` (`self.InteractTooltip1`) false false)))
    (elif (`self.Is Closed`)
      (set `self.Is Closed` false :!label _label)
      (`self.DisableInput` (`GameplayStatics.GetPlayerController` 0))
      (`KismetSystemLibrary.MoveComponentTo` (`self.Cube`) (140.0 -30.0 200.0) (struct :`Yaw` 90.0) true true _returnvalue)
      (`self.EnableInput` (`GameplayStatics.GetPlayerController` 0))
      (`KismetSystemLibrary.MoveComponentTo` (`self.Box`) (150.0 -30.0 220.0) (struct) false false _returnvalue)
      (`SceneComponent.SetVisibility` (`self.InteractTooltip`) false false)
      (`SceneComponent.SetVisibility` (`self.InteractTooltip1`) false false))))

(event `InputAction|Interact`
  (params (Key :type "Key Structure"))
  (bind _returnvalue (`KismetMathLibrary.SelectFloat` 2.0 0.5 (`self.Underwater`)))
  (:`Pressed`
    (if (`self.In Range`)
      (if (`self.Is Closed`)
        (goto _label)
        (else
          (set `self.Is Closed` true)
          (`self.DisableInput` (`GameplayStatics.GetPlayerController` 0))
          (`KismetSystemLibrary.MoveComponentTo` (`self.Cube`) (-10.0 -180.0 200.0) (struct) false true _returnvalue)
          (`self.EnableInput` (`GameplayStatics.GetPlayerController` 0))
          (`KismetSystemLibrary.MoveComponentTo` (`self.Box`) (0.0 -180.0 220.0) (struct) false false _returnvalue)
          (`SceneComponent.SetVisibility` (`self.InteractTooltip`) false false)
          (`SceneComponent.SetVisibility` (`self.InteractTooltip1`) false false))))))

(fn `UserConstructionScript`)